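; Drivable jeep vehicle that the top-down player can board and exit.
; Enhanced Input move axes feed steering and throttle on the vehicle movement component.
; Possession shows the driver mesh with an enter montage; the pick-up input plays an exit montage, then hides the mesh and has BP_TopDownController depossess the jeep.
; The PlayerDetection overlap sets ReadyForPlayer while BP_TopDownCharacter is in range.
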(event `OnPossess`
  (bind _drivermesh (`self.DriverMesh`))
  (`SceneComponent.SetVisibility` _drivermesh true false)
  (`|PlayMontage` _drivermesh (`self.EnterJeepMontage`)))

(event `self.ReceiveBeginPlay`
  (`EnhancedInputSubsystemInterface.AddMappingContext` (pcsubsystem `EnhancedInputLocalPlayerSubsystem` (`GameplayStatics.GetPlayerController` 0)) "/Game/TopDown/Input/IMC_Default.IMC_Default" 0 (struct)))

(event `EnhancedInput|/Game/TopDown/Input/Actions/IA_Move`
  (params (ActionValue :type "Vector2D Structure") (ElapsedSeconds :type "Float (double-precision)") (TriggeredSeconds :type "Float (double-precision)") (InputAction :type "InputAction Object Reference" :default "/Game/TopDown/Input/Actions/IA_Move.IA_Move"))
  (bind _vehiclemovementcomponent (`self.VehicleMovementComponent`))
  (:`Triggered`
    (`|ExecutionSequence` :!label _label
      (:`then_0`
        (`ChaosVehicleMovementComponent.SetSteeringInput` _vehiclemovementcomponent ActionValue_Y))
      (:`then_1`
        (`ChaosVehicleMovementComponent.SetThrottleInput` _vehiclemovementcomponent ActionValue_X))))
  (:`Canceled`
    (goto _label))
  (:`Completed`
    (goto _label)))

(event `EnhancedInput|/Game/pick_up_folder/IA_PickUp`
  (params (ActionValue :type Boolean) (ElapsedSeconds :type "Float (double-precision)") (TriggeredSeconds :type "Float (double-precision)") (InputAction :type "InputAction Object Reference" :default "/Game/pick_up_folder/IA_PickUp.IA_PickUp"))
  (bind _drivermesh (`self.DriverMesh`))
  (:`Started`
    (bind _asbp_top_down_controller (cast `/Game/TopDown/Blueprints/BP_TopDownController` (`self.GetController`)))
    (`|PlayMontage` _drivermesh (`self.ExitJeepMontage`)
      (:`OnCompleted`
        (`SceneComponent.SetVisibility` _drivermesh false false)
        (`/Game/TopDown/Blueprints/BP_TopDownController.DepossessJeep` _asbp_top_down_controller self)))))

(event `self.PlayerDetection.OnComponentBeginOverlap`
  (params (OverlappedComponent :type "PrimitiveComponent Object Reference") (OtherActor :type "Actor Object Reference") (OtherComp :type "PrimitiveComponent Object Reference") (OtherBodyIndex :type Integer) (bFromSweep :type Boolean) (SweepResult :type "HitResult Structure (by ref)"))
  (cast `/Game/TopDown/Blueprints/BP_TopDownCharacter` OtherActor)
  (set `self.ReadyForPlayer` true))

(event `self.PlayerDetection.OnComponentEndOverlap`
  (params (OverlappedComponent :type "PrimitiveComponent Object Reference") (OtherActor :type "Actor Object Reference") (OtherComp :type "PrimitiveComponent Object Reference") (OtherBodyIndex :type Integer))
  (cast `/Game/TopDown/Blueprints/BP_TopDownCharacter` OtherActor)
  (set `self.ReadyForPlayer` false))

(fn `UserConstructionScript`)