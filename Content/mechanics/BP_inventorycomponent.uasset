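; Inventory component that holds a ten-slot item array, creates the inventory widget on BeginPlay and toggles it with I.
; E runs a debug-drawn sphere trace at player 0's feet to pick up a BP_item.
; The item goes into the first slot that is either empty or a matching stackable stack staying within 64.
; A successful pickup reloads the widget and destroys the actor, whose validity check guards later loop iterations.
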(event `self.ReceiveBeginPlay`
  (bind _returnvalue (`|CreateWidget` "/Game/inventory/widgets/WB_inventory.WB_inventory_C"))
  (set `self.inventorywidget` _returnvalue)
  (`KismetArrayLibrary.Array_Resize` (`self.items`) 10)
  (`/Game/inventory/widgets/WB_inventory.loadinventory` (`self.inventorywidget`) self))

(event `Key|I`
  (params (Key :type "Key Structure"))
  (bind _inventorywidget (`self.inventorywidget`))
  (:`Pressed`
    (if (`Widget.IsVisible` (`self.inventorywidget`))
      (`Widget.RemoveFromParent` _inventorywidget)
      (else
        (`UserWidget.AddToViewport` _inventorywidget 0)))))

(event `Key|E`
  (params (Key :type "Key Structure"))
  (bind _returnvalue (- (`Actor.K2_GetActorLocation` (`GameplayStatics.GetPlayerCharacter` 0)) (0.0 0.0 65.0)))
  (:`Pressed`
    (bind _outhit (`KismetSystemLibrary.SphereTraceSingle` :`Start` _returnvalue :`End` _returnvalue :`Radius` 120.0 :`TraceChannel` "TraceTypeQuery1" :`DrawDebugType` "ForDuration"))
    (bind _asbp_item (cast `/Game/inventory/blueprints/BP_item` (`.HitActor` (`GameplayStatics.BreakHitResult` _outhit))))
    (for (_array_element _array_index) (`self.items`)
      (`/Engine/EditorBlueprintResources/StandardMacros.IsValid` _asbp_item
        (:`Is Valid`
          (bind (_item _stackable _quantity) (break `/Game/inventory/blueprints/S_itemstructure` _array_element))
          (bind (_item_2 _stackable_2 _quantity_2) (break `/Game/inventory/blueprints/S_itemstructure` (`/Game/inventory/blueprints/BP_item.item` _asbp_item)))
          (bind _returnvalue_2 (+ _quantity _quantity_2))
          (if (and (`KismetTextLibrary.EqualEqual_TextText` _item _item_2) _stackable_2 (<= _returnvalue_2 64))
            (bind (_item_item _item_stackable _item_quantity _item_thumbnail _item_mesh) (break `/Game/inventory/blueprints/S_itemstructure` (`/Game/inventory/blueprints/BP_item.item` _asbp_item)))
            (`KismetArrayLibrary.Array_Set` (`self.items`) _array_index (make `/Game/inventory/blueprints/S_itemstructure` _item_item _item_stackable _returnvalue_2 _item_thumbnail _item_mesh))
            (`/Game/inventory/widgets/WB_inventory.loadinventory` (`self.inventorywidget`) self :!label _label)
            (`Actor.K2_DestroyActor` _asbp_item)
            (elif (== _quantity 0)
              (`KismetArrayLibrary.Array_Set` (`self.items`) _array_index (`/Game/inventory/blueprints/BP_item.item` _asbp_item))
              (goto _label))))))))